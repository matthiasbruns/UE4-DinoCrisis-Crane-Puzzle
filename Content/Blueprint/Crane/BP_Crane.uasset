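; Card-programmed crane that runs the player's selected movement and hook cards in sequence to carry crates.
; HandleCraneStep chains cards through timelines that lerp the hook to destinations from NextDestination.
; Both hook cards dip and return, enabling collision at the bottom; overlap attaches a crate, HOOK_DOWN releases it.
; Crate collision, leaving bounds or finishing calls HandleCraneStop, which returns the hook home and clears selection, with dispatchers reporting progress.
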(event `self.HookCollision.OnComponentBeginOverlap`
  (params (OverlappedComponent :type "PrimitiveComponent Object Reference") (OtherActor :type "Actor Object Reference") (OtherComp :type "PrimitiveComponent Object Reference") (OtherBodyIndex :type Integer) (bFromSweep :type Boolean) (SweepResult :type "HitResult Structure (by ref)"))
  ;[1 0.3305 0.2207] Attach crate to hook when coliding
  (`/Engine/EditorBlueprintResources/StandardMacros.IsValid` (`self.AttachedCrate`)
    (:`Is Not Valid`
      (bind _asbp_crate (cast `/Game/Blueprint/Crane/BP_Crate` OtherActor))
      (`self.K2_AttachToComponent` _asbp_crate (`self.CraneSocket`) "None" "KeepWorld" "KeepRelative" "KeepRelative" true)
      (bind _output_get (set `self.AttachedCrate` _asbp_crate))
      (add `/Game/Blueprint/Crane/BP_Crate.OnOtherCrateCollision` _output_get (delegate `OnOtherCreateCollision_Event`)))))

(event `OnOtherCreateCollision_Event`
  ;[1 0.3305 0.2207] Attach crate to hook when coliding
  (`self.HandleCraneStop`))

(event `HandleCraneStep`
  (params (index :type Integer))
  (bind _output (`|GetArrayItem` (`self.SelectedCards`) index))
  (bind (_type _steps) (break `/Game/Blueprint/Crane/BP_CraneCard` _output))
  (set `self.CurrentIndex` index)
  ;[0.4078 0.1412 0.2784] Check if index is valid and store current hook position
  (if (`KismetArrayLibrary.Array_IsValidIndex` (`self.SelectedCards`) index)
    (bind _output_get (set `self.LastHookPosition` (`SceneComponent.RelativeLocation` (`self.HookRoot`))))
    (set `self.CurrentCard` _output)
    (`self.OnCraneStep`)
    (switch `/Game/Blueprint/Crane/BP_CraneCardType` _type
      (:`NewEnumerator0`
        (bind _destination (`self.Next Destination` _output_get _type _steps))
        ;[0.4078 0.1412 0.2784] Unidirectional movement for UP, DOWN, LEFT, RIGHT
        (set `self.NextHookPosition` _destination :!label _label)
        (bind (_direction _alpha) (`Timeline|HookMovementTimeline` :`NewTime` 0.5 :!via `PlayFromStart`)
          (:`Update`
            (`SceneComponent.K2_SetRelativeLocation` (`self.HookRoot`) (`KismetMathLibrary.VLerp` (`self.LastHookPosition`) (`self.NextHookPosition`) _alpha) false false))
          (:`Finished`
            ;[0.4078 0.1412 0.2784] Increment card index and decide the sequence is done or continue
            (bind _result (`/Engine/EditorBlueprintResources/StandardMacros.IncrementInt` (`self.CurrentIndex`) :!label _label_2)
              (:`  `
                (if (>= _result (`KismetArrayLibrary.Array_Length` (`self.SelectedCards`)))
                  (`self.HandleCraneStop`)
                  (else
                    (`self.HandleCraneStep` _result))))))))
      (:`NewEnumerator1`
        (goto _label))
      (:`NewEnumerator2`
        (goto _label))
      (:`NewEnumerator3`
        (goto _label))
      (:`NewEnumerator4`
        ;[0.4078 0.1412 0.2784] Disable collision when going UP or DOWN
        (`PrimitiveComponent.SetCollisionEnabled` (`self.HookCollision`) "NoCollision" :!label _label_3)
        ;[0.4078 0.1412 0.2784] Move UP or DOWN and enable collision afterwards
        (set `self.NextHookPosition` _destination)
        (bind (_direction_2 _alpha_2) (`Timeline|HookUpDownTimeline` :!via `PlayFromStart`)
          (:`Update`
            (`SceneComponent.K2_SetRelativeLocation` (`self.HookRoot`) (`KismetMathLibrary.VLerp` (`self.LastHookPosition`) (`self.NextHookPosition`) _alpha_2) false false))
          (:`Finished`
            (`PrimitiveComponent.SetCollisionEnabled` (`self.HookCollision`) "QueryOnly")
            (if (and (`|EnumEquality` (`.Type_3_021D6EF841E0DA7538A656A06D59D421` (break `/Game/Blueprint/Crane/BP_CraneCard` (`self.CurrentCard`))) "NewEnumerator5") (`KismetSystemLibrary.IsValid` (`self.AttachedCrate`)))
              ;[0.4078 0.1412 0.2784] Detach crate and reset listeners when direction is DOWN after moving downwards
              (`self.K2_DetachFromActor` (`self.AttachedCrate`) "KeepWorld" "KeepRelative" "KeepRelative")
              (clear `/Game/Blueprint/Crane/BP_Crate.OnOtherCrateCollision` (`self.AttachedCrate`))
              (set `self.AttachedCrate` null)
              ;[0.4078 0.1412 0.2784] Reverse movement of UP and DOWN after previous movement to reset position
              (bind (_direction_3 _alpha_3) (`Timeline|HookUpDownRevTimeline` :!via `PlayFromStart` :!label _label_4)
                (:`Update`
                  (`SceneComponent.K2_SetRelativeLocation` (`self.HookRoot`) (`KismetMathLibrary.VLerp` (`self.NextHookPosition`) (`self.LastHookPosition`) _alpha_3) false false))
                (:`Finished`
                  (goto _label_2)))
              (else
                (goto _label_4 :!via `PlayFromStart`))))))
      (:`NewEnumerator5`
        (goto _label_3)))))

(event `HandleCraneStop`
  (`|ExecutionSequence`
    (:`then_0`
      ;[0.6599 1 0.7731] Stop crane movement
      (`TimelineComponent.Stop` (`self.HookMovementTimeline`))
      (`TimelineComponent.Stop` (`self.HookUpDownTimeline`))
      (`TimelineComponent.Stop` (`self.HookUpDownRevTimeline`)))
    (:`then_1`
      ;[0.2462 0.3763 0.2918] Reset card and index caching
      (set `self.CurrentIndex` -1)
      (set `self.CurrentCard` (struct)))
    (:`then_2`
      ;[0.0999 0.1529 0.1195] Move crane to starting position
      (bind _output_get (set `self.LastHookPosition` (`SceneComponent.RelativeLocation` (`self.HookRoot`))))
      (bind (_direction _alpha) (`Timeline|ResetCraneTimeline` :!via `PlayFromStart`)
        (:`Update`
          (`SceneComponent.K2_SetRelativeLocation` (`self.HookRoot`) (`KismetMathLibrary.VLerp` _output_get (`self.StartHookPosition`) _alpha) false false))
        (:`Finished`
          (`self.ResetCards`)
          (`self.OnCraneStopped`))))))

(event `self.CraneBoundsBox.OnComponentEndOverlap`
  (params (OverlappedComponent :type "PrimitiveComponent Object Reference") (OtherActor :type "Actor Object Reference") (OtherComp :type "PrimitiveComponent Object Reference") (OtherBodyIndex :type Integer))
  (bind _hookcollision (`self.HookCollision`))
  ;[1 0.4362 0.4163] Handle out of bounds and reset crane
  (if (and (`PrimitiveComponent.K2_IsCollisionEnabled` _hookcollision) (== OtherComp _hookcollision))
    (`self.HandleCraneStop`)))

(fn `CanStart`
  (returns (ReturnValue :type Boolean))
  (return (> (`KismetArrayLibrary.Array_Length` (`self.SelectedCards`)) 0)))

(fn `CraneStepIndex`
  (returns (Index :type Integer))
  (return (`self.CurrentIndex`)))

(fn `Next Destination`
  (params (StartPosition :type "Vector Structure") (CardType :type "/Game/Blueprint/Crane/BP_CraneCardType Enum" :default "NewEnumerator0") (Steps :type Integer))
  (returns (Destination :type "Vector Structure"))
  (switch `/Game/Blueprint/Crane/BP_CraneCardType` CardType
    (:`NewEnumerator0`
      (return (+ StartPosition (* (`KismetMathLibrary.MakeVector` 200.0) Steps))))
    (:`NewEnumerator1`
      (return (+ StartPosition (* (`KismetMathLibrary.MakeVector` -200.0) Steps))))
    (:`NewEnumerator2`
      (return (+ StartPosition (* (`KismetMathLibrary.MakeVector` 0.0 -100.0) Steps))))
    (:`NewEnumerator3`
      (return (+ StartPosition (* (`KismetMathLibrary.MakeVector` 0.0 100.0) Steps))))
    (:`NewEnumerator4`
      (return (+ StartPosition (* (`KismetMathLibrary.MakeVector` 0.0 0.0 -120.0) Steps))))
    (:`NewEnumerator5`
      (return (+ StartPosition (* (`KismetMathLibrary.MakeVector` 0.0 0.0 -120.0) Steps))))))

(fn `ResetCards`
  (locals (CardLength :type Integer))
  (bind _output_get (set `local.CardLength` (`KismetArrayLibrary.Array_Length` (`self.SelectedCards`))))
  (`KismetArrayLibrary.Array_Clear` (`self.SelectedCards`))
  (if (> _output_get 0)
    (`self.OnCardSelectionChanged`)))

(fn `Start`
  (if (`self.CanStart`)
    (`self.OnCraneStarted`)
    (`self.HandleCraneStep` 0)))

(fn `ToggleCard`
  (params (Card :type "/Game/Blueprint/Crane/BP_CraneCard Structure"))
  (if (`KismetArrayLibrary.Array_Contains` (`self.SelectedCards`) Card)
    (bind _returnvalue (`KismetArrayLibrary.Array_RemoveItem` (`self.SelectedCards`) Card))
    (if _returnvalue
      (`self.OnCardSelectionChanged` :!label _label))
    (else
      (bind _returnvalue_2 (`KismetArrayLibrary.Array_AddUnique` (`self.SelectedCards`) Card))
      (if (`KismetArrayLibrary.Array_IsValidIndex` (`self.SelectedCards`) _returnvalue_2)
        (goto _label)))))

(fn `UserConstructionScript`
  (set `self.Cards` (`|MakeArray` (make `/Game/Blueprint/Crane/BP_CraneCard` "NewEnumerator3" 2) (make `/Game/Blueprint/Crane/BP_CraneCard` "NewEnumerator1") (make `/Game/Blueprint/Crane/BP_CraneCard` "NewEnumerator2") (make `/Game/Blueprint/Crane/BP_CraneCard` "NewEnumerator0" 2) (make `/Game/Blueprint/Crane/BP_CraneCard` "NewEnumerator4") (make `/Game/Blueprint/Crane/BP_CraneCard` "NewEnumerator5")))
  (`SceneComponent.K2_SetRelativeLocation` (`self.HookRoot`) (`self.StartHookPosition`) false false)
  (`SceneComponent.SetRelativeScale3D` (`self.CraneBoundsBox`) (`self.CraneBounds`)))